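; BP_Finish is the level finish trigger, ending the level when BP_ThirdPersonCharacter overlaps its Box.
; The overlap plays a sound, sets Finish on BP_PlatformGameMode and removes that game mode's HUD widget.
; It then disables character movement and switches to UI-only input with a visible cursor.
; WBP_LevelComplete is created and added to the viewport twice, before and after movement is disabled, so two copies stack.
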(event OnComponentBeginOverlap(Box)
  (params (OverlappedComponent :type Primitive%20Component%20Object%20Reference) (OtherActor :type Actor%20Object%20Reference) (OtherComp :type Primitive%20Component%20Object%20Reference) (OtherBodyIndex :type Integer) (bFromSweep :type Boolean) (SweepResult :type Hit%20Result%20Structure%20%28by%20ref%29))
  ;[0.15 0.15 0.15 0.5] Set Finish True
  (bind _asbp_third_person_character (Utilities|Casting|CastToBP_ThirdPersonCharacter OtherActor))
  (Audio|PlaySound2D "/Game/Sounds/SciFiUISFX/Wavs/Glitches/Glitch_10_Wav.Glitch_10_Wav" 1.0 1.0 0.0 0 0)
  (bind _asbp_platform_game_mode (Utilities|Casting|CastToBP_PlatformGameMode (Game|GetGameMode)))
  (Variables|/Game/Blueprints/BP_PlatformGameMode.BP_PlatformGameMode_C|SetFinish _asbp_platform_game_mode true)
  ;[0.15 0.15 0.15 0.5] Level Complete Widget
  (bind _asbp_platform_game_mode_2 (Utilities|Casting|CastToBP_PlatformGameMode (Game|GetGameMode)))
  (Widget|RemovefromParent (Variables|/Game/Blueprints/BP_PlatformGameMode.BP_PlatformGameMode_C|GetHUDWidget _asbp_platform_game_mode_2))
  (bind _returnvalue (UserInterface|CreateWidget "/Game/Blueprints/WBP_LevelComplete.WBP_LevelComplete_C" (Game|GetPlayerController 0)))
  (UserInterface|Viewport|AddtoViewport _returnvalue 0)
  ;[0.15 0.15 0.15 0.5] Disable Movement in Finish
  (Pawn|Components|CharacterMovement|SetMovementMode (Variables|/Script/Engine.Character|GetCharacterMovement _asbp_third_person_character) "MOVE_None" 0)
  (bind _returnvalue_2 (UserInterface|CreateWidget "/Game/Blueprints/WBP_LevelComplete.WBP_LevelComplete_C" (Game|GetPlayerController 0)))
  (UserInterface|Viewport|AddtoViewport _returnvalue_2 0)
  (Input|SetInputModeUIOnly (Game|GetPlayerController 0) 0 "DoNotLock" false)
  (Variables|/Script/Engine.PlayerController|SetbShowMouseCursor (Game|GetPlayerController 0) true))

(fn ConstructionScript)