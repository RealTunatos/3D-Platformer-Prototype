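; BP_PlatformGameMode is a game mode for a platforming level that sets up the HUD and runs a level timer.
; On BeginPlay it creates and stores a WBP_HUD widget, adds it to the viewport, switches input to game-only and hides the mouse cursor.
; Each Tick it adds DeltaSeconds to ElapsedTime until the Finish flag is set.
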(event EventTick
  (params (DeltaSeconds :type Float%20%28single-precision%29))
  ;[0.15 0.15 0.15 0.5] Timer Function
  (if (not (Variables|Default|GetFinish))
    (Variables|Default|SetElapsedTime (+ (Variables|Default|GetElapsedTime) DeltaSeconds))))

(event EventBeginPlay
  (bind _returnvalue (Game|GetPlayerController 0))
  ;[0.15 0.15 0.15 0.5] Timer Widget
  (bind _returnvalue_2 (UserInterface|CreateWidget "/Game/Blueprints/WBP_HUD.WBP_HUD_C" (Game|GetPlayerController 0)))
  (bind _output_get (Variables|Default|SetHUDWidget _returnvalue_2))
  (UserInterface|Viewport|AddtoViewport _output_get 0)
  (Input|SetInputModeGameOnly _returnvalue false)
  (Variables|/Script/Engine.PlayerController|SetbShowMouseCursor _returnvalue false))

(fn ConstructionScript)